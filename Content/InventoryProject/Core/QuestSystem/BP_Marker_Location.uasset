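; BP_Marker_Location is a quest marker actor that reports when the player reaches a location.
; On sphere overlap by BP_PlayerCharacter, it scans the quest log component's quests and their objectives.
; For each incomplete, completable Location-type objective, it calls CallLocationReached on that quest, passing itself.
; A debug print is left unconnected.
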(event OnComponentBeginOverlap(Sphere)
  (params (OverlappedComponent :type Primitive%20Component%20Object%20Reference) (OtherActor :type Actor%20Object%20Reference) (OtherComp :type Primitive%20Component%20Object%20Reference) (OtherBodyIndex :type Integer) (bFromSweep :type Boolean) (SweepResult :type Hit%20Result%20Structure%20%28by%20ref%29))
  (bind _asbp_player_character (Utilities|Casting|CastToBP_PlayerCharacter OtherActor))
  (for _array_element (Variables|/Game/InventoryProject/Core/QuestSystem/BP_Quest_LogComponent.BP_Quest_LogComponent_C|GetQuests (Variables|/Game/InventoryProject/Core/Characters/BP_PlayerCharacter.BP_PlayerCharacter_C|GetBP_Quest_LogComponent _asbp_player_character))
    ;[1 1 1] Check whether objective is of Location type and hasn't been completed already
    (for _array_element_2 (Variables|/Game/InventoryProject/Core/QuestSystem/Quests/BP_Quest.BP_Quest_C|GetObjectives _array_element)
      (if (Math|Boolean|ANDBoolean (Utilities|Enum|Equal(Enum) (.Type (Utilities|Struct|BreakFObjective_Data _array_element_2)) "NewEnumerator0") (not (.bCompleted (Utilities|Struct|BreakFObjective_Data _array_element_2))) (.bCanBeCompleted (Utilities|Struct|BreakFObjective_Data _array_element_2)))
        (Default|CallLocationReached _array_element self)))))

(fn ConstructionScript)