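; Quest log component that stores the player's current and completed quests, tracks the active one and toggles the quest log widget.
; Changing the active quest refreshes HUD objectives and, with the log open, re-evaluates collect objectives through player inventory queries.
; Deleting a quest archives it if completed or resets objectives if abandoned, then activates the first remaining quest.
; Completed quests are only printed as debug strings, and deprecated collect-objective logic remains unconnected.
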(event EventBeginPlay
  (Variables|Default|SetPlayerRef (.AsBP%20Player%20Character (Utilities|Casting|CastToBP_PlayerCharacter (Game|GetPlayerCharacter 0)))))

(fn AddQuesttoLog
  (params (Quest :type BP%20Quest%20Object%20Reference))
  ;[1 1 1] Double check if player already has this quest
  (if (not (Utilities|Array|ContainsItem (Variables|Default|GetQuests) Quest))
    (Utilities|Array|AddUnique (Variables|Default|GetQuests) Quest)))

(fn ToggleQuestLog
  (bind _returnvalue (Game|GetPlayerController 0))
  (bind _quest_log_ref (Variables|Default|GetQuest%20Log%20Ref)
    (:then
      (Widget|RemovefromParent _quest_log_ref)
      (Variables|Default|SetQuest%20Log%20Ref 0)
      (Default|SetDefaultInputMode (.AsPC%20Main (Utilities|Casting|CastToPC_Main _returnvalue))))
    (:else
      (bind _returnvalue_2 (UserInterface|CreateWidget "/Game/InventoryProject/Core/QuestSystem/UI/WBP_Quest_Log.WBP_Quest_Log_C"))
      (bind _output_get (Variables|Default|SetQuest%20Log%20Ref _returnvalue_2))
      (UserInterface|Viewport|AddtoViewport _output_get 0)
      (Input|SetInputModeUIOnly _returnvalue _returnvalue_2 "LockAlways")
      (Variables|/Script/Engine.PlayerController|SetbShowMouseCursor _returnvalue true))))

(fn SetActiveQuest
  (params (Quest :type BP%20Quest%20Object%20Reference) (bPlaySound :type Boolean))
  ;[1 1 1] Set player's active quest
  (Variables|Default|SetActiveQuest Quest)
  ;[1 1 1] Update quest's objectives in HUD
  (Default|UpdateObjectivesList (Variables|/Game/InventoryProject/Core/UI/WBP_HUD.WBP_HUD_C|GetWBP_Quest_HUD_Objectives (Variables|/Game/InventoryProject/Core/PlayerControllers/PC_Main.PC_Main_C|GetHUD_Reference (.AsPC%20Main (Utilities|Casting|CastToPC_Main (Game|GetPlayerController 0))))))
  ;[1 1 1] Set quest's objectives in Quest Log (providing there is a valid Quest Log)
  (bind _quest_log_ref (Variables|Default|GetQuest%20Log%20Ref)
    (:then
      (Default|OnActiveQuestChanged _quest_log_ref)
      ;[1 1 1] Update Collect objectives
      (CallFunction|CheckPlayerInventory (Variables|Default|GetActiveQuest))
      (CallFunction|IsQuestCompleted (Variables|Default|GetActiveQuest)))
    (:else
      _))
  ;[1 1 1] Play sound if need
  (if bPlaySound
    (Audio|PlaySound2D "/Game/InventoryProject/Sounds/Interface/Quests/A_UI_Quest_Update.A_UI_Quest_Update" 0.8 1.0 0.0 0 0)))

(fn DeleteQuest
  (params (Quest :type BP%20Quest%20Object%20Reference%20%28by%20ref%29) (bWasQuestAbandoned :type Boolean))
  (bind _objectives (Variables|/Game/InventoryProject/Core/QuestSystem/Quests/BP_Quest.BP_Quest_C|GetObjectives Quest))
  (bind _quest_log_ref (Variables|Default|GetQuest%20Log%20Ref))
  (bind _quests (Variables|Default|GetQuests))
  (Utilities|FlowControl|Sequence
    (:then_0
      ;[1 1 1] Add completed quest to complete quest list
      (if (Variables|/Game/InventoryProject/Core/QuestSystem/Quests/BP_Quest.BP_Quest_C|GetbCompleted Quest)
        (Utilities|Array|AddUnique (Variables|Default|GetQuests_Completed) Quest)))
    (:then_1
      ;[1 1 1] Abandon the quest. Mark all objectives as incomplete, remove quest entry from quest log, play sound
      (if bWasQuestAbandoned
        (Variables|/Game/InventoryProject/Core/QuestSystem/Quests/BP_Quest.BP_Quest_C|SetbCompleted Quest false)
        (for (_array_element _array_index) _objectives
          (Utilities|Array|SetArrayElem _objectives _array_index (Utilities|Struct|MakeFObjective_Data (.Description (Utilities|Struct|BreakFObjective_Data _array_element)) (.Type (Utilities|Struct|BreakFObjective_Data _array_element)) false false (.Target (Utilities|Struct|BreakFObjective_Data _array_element)) (.Amount (Utilities|Struct|BreakFObjective_Data _array_element)))))
        (Class|PanelWidget|RemoveChild (Variables|/Game/InventoryProject/Core/QuestSystem/UI/WBP_Quest_Log.WBP_Quest_Log_C|GetQuests_Side _quest_log_ref) (Variables|/Game/InventoryProject/Core/QuestSystem/Quests/BP_Quest.BP_Quest_C|GetQuestLogEntryRef Quest))
        (Class|PanelWidget|RemoveChild (Variables|/Game/InventoryProject/Core/QuestSystem/UI/WBP_Quest_Log.WBP_Quest_Log_C|GetQuests_Story _quest_log_ref) (Variables|/Game/InventoryProject/Core/QuestSystem/Quests/BP_Quest.BP_Quest_C|GetQuestLogEntryRef Quest))
        (Variables|/Game/InventoryProject/Core/QuestSystem/Quests/BP_Quest.BP_Quest_C|SetQuestLogEntryRef Quest 0)
        (Audio|PlaySound2D "/Game/InventoryProject/Sounds/Interface/Quests/A_UI_Quest_Failed.A_UI_Quest_Failed" 1.0 1.0 0.0 0 0)))
    (:then_2
      ;[1 1 1] Remove quest from log and ui, set new active quest if quest log is not empty
      ;;[1 1 1] Remove quest from list and update UI
      (Utilities|Array|RemoveItem _quests Quest)
      (CallFunction|SetActiveQuest 0 false)
      (if (Utilities|Array|IsNotEmpty _quests) ; Check if quest list is not empty
        ;;[1 1 1] Find first valid quest and set it to Active
        (bind _index (Utilities|FlowControl|ForLoopwithBreak 0 (Utilities|Array|Length _quests) :!label _label)
          (:LoopBody
            (if (Utilities|Array|IsValidIndex _quests _index)
              (LocalVariables|SetbFoundFirstValidIndex true)
              (LocalVariables|SetFirstValidIndex _index)
              (goto _label Break)))
          (:Completed
            (if (LocalVariables|GetbFoundFirstValidIndex)
              (CallFunction|SetActiveQuest (Utilities|Array|Get(acopy) _quests (LocalVariables|GetFirstValidIndex)) false))))
        (else
          ;[1 1 1] Remove everything from description box (quest name, quest description, rewards) if no quests left in quest log while it is open
          (bind _quest_log_ref_2 (Variables|Default|GetQuest%20Log%20Ref)
            (:then
              (Widget|Panel|ClearChildren (Variables|/Game/InventoryProject/Core/QuestSystem/UI/WBP_Quest_Log.WBP_Quest_Log_C|GetVerticalBox_Quest_Desc _quest_log_ref_2))
              ;[1 1 1] Set abandon quest button visibility to hidden
              (Variables|/Game/InventoryProject/Core/QuestSystem/UI/WBP_Quest_Log.WBP_Quest_Log_C|SetActive%20Quest _quest_log_ref_2 0)
              (Default|CheckButtonAbandonVisibility _quest_log_ref_2))
            (:else)))))))

(fn GetCompletedQuests
  (bind _quests_completed (Variables|Default|GetQuests_Completed))
  (if (Utilities|Array|IsNotEmpty _quests_completed)
    (bind (_arrayindex _arrayelement) (Utilities|Array|ReverseforEachLoop _quests_completed) ; Use reverse so we could get elements of a list in order from 0 to N (rather then vise versa)
      (:LoopBody
        (LocalVariables|SetQuestIndex _arrayindex)
        (Development|PrintString (Utilities|String|Append (Utilities|String|ToString(Integer) (+ (LocalVariables|GetQuestIndex) 1)) ": " (Utilities|String|ToString(Text) (Variables|/Game/InventoryProject/Core/QuestSystem/Quests/BP_Quest.BP_Quest_C|GetName _arrayelement))))))
    (else
      (bind _returnvalue (UserInterface|CreateWidget "/Game/InventoryProject/Core/UI/WBP_Message_Error.WBP_Message_Error_C" 0 "You haven't completed any quests yet!"))
      (UserInterface|Viewport|AddtoViewport _returnvalue 0))))

(fn CheckPlayerInventory
  (params (Quest :type BP%20Quest%20Object%20Reference))
  (bind _indicesofsuccessfullyqueriedobjectives (LocalVariables|GetIndicesOfSuccessfullyQueriedObjectives))
  (bind _objectives (Variables|/Game/InventoryProject/Core/QuestSystem/Quests/BP_Quest.BP_Quest_C|GetObjectives Quest))
  (bind (_array_element _array_index) (Utilities|Array|ForEachLoopwithBreak (Variables|/Game/InventoryProject/Core/QuestSystem/Quests/BP_Quest.BP_Quest_C|GetObjectives Quest))
    (:LoopBody
      (if (Utilities|Enum|Equal(Enum) (.Type (Utilities|Struct|BreakFObjective_Data _array_element)) "NewEnumerator2")
        (bind _asbp_item (Utilities|Casting|CastToBP_Item (.Target (Utilities|Struct|BreakFObjective_Data _array_element))))
        (LocalVariables|SetbCollectableObjectiveExists true)
        ;[1 1 1] Save all Collect objectives, their indices and Inventory query status of quest items they represent
        (Utilities|Array|AddUnique (LocalVariables|GetObjectiveElement) _array_element)
        (bind _bisininventory (Default|InventoryQuery (Variables|/Game/InventoryProject/Core/Characters/BP_PlayerCharacter.BP_PlayerCharacter_C|GetBP_InventoryComponent (Variables|Default|GetPlayerRef)) (Utilities|GetClass _asbp_item) (.Amount (Utilities|Struct|BreakFObjective_Data _array_element))))
        (Utilities|Map|Add (LocalVariables|GetIndicesOfSuccessfullyQueriedObjectives) _array_index _bisininventory)))
    (:Completed
      (if (LocalVariables|GetbCollectableObjectiveExists) ; Check if quest has at least one Collect objective
        ;[1 1 1] Seems to be working perfectly no matter the order of Collect objectives. We use map's keys for primary for each loop, passing array element (what's situated on index) as index for element of the objectives array, then we use keys array index as index for value to check, and if that value is True - we actually set the array element with previously saved objective from the same index but changing only completion status. We do this for each Collect objective, no matter the index in objective array. I know that sound extremely confusing but just try and understand
        (bind _keys (Utilities|Map|Keys _indicesofsuccessfullyqueriedobjectives))
        (for (_array_element_2 _array_index_2) _keys
          (bind _values (Utilities|Map|Values _indicesofsuccessfullyqueriedobjectives))
          (if (Utilities|Array|Get(acopy) _values _array_index_2)
            (Utilities|Array|SetArrayElem _objectives _array_element_2 (Utilities|Struct|MakeFObjective_Data (.Description (Utilities|Struct|BreakFObjective_Data (Utilities|Array|Get(acopy) (LocalVariables|GetObjectiveElement) _array_index_2))) (.Type (Utilities|Struct|BreakFObjective_Data (Utilities|Array|Get(acopy) (LocalVariables|GetObjectiveElement) _array_index_2))) true true (.Target (Utilities|Struct|BreakFObjective_Data (Utilities|Array|Get(acopy) (LocalVariables|GetObjectiveElement) _array_index_2))) (.Amount (Utilities|Struct|BreakFObjective_Data (Utilities|Array|Get(acopy) (LocalVariables|GetObjectiveElement) _array_index_2)))))
            (else
              (Utilities|Array|SetArrayElem _objectives _array_element_2 (Utilities|Struct|MakeFObjective_Data (.Description (Utilities|Struct|BreakFObjective_Data (Utilities|Array|Get(acopy) (LocalVariables|GetObjectiveElement) _array_index_2))) (.Type (Utilities|Struct|BreakFObjective_Data (Utilities|Array|Get(acopy) (LocalVariables|GetObjectiveElement) _array_index_2))) false false (.Target (Utilities|Struct|BreakFObjective_Data (Utilities|Array|Get(acopy) (LocalVariables|GetObjectiveElement) _array_index_2))) (.Amount (Utilities|Struct|BreakFObjective_Data (Utilities|Array|Get(acopy) (LocalVariables|GetObjectiveElement) _array_index_2))))))))))))

(fn IsQuestCompleted
  (params (Quest :type BP%20Quest%20Object%20Reference))
  ;[1 1 1] If at least one of the objectives is not complete - quest isn't complete aswell (bAllObjectivesComplete = false), otherwise - quest is complete
  (for _array_element (Variables|/Game/InventoryProject/Core/QuestSystem/Quests/BP_Quest.BP_Quest_C|GetObjectives Quest)
    (if (not (.bCompleted (Utilities|Struct|BreakFObjective_Data _array_element)))
      (LocalVariables|SetbAllObjectivesCompleted false)))
  (return (LocalVariables|GetbAllObjectivesCompleted)))