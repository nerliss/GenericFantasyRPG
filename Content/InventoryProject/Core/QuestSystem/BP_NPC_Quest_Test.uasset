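; BP_NPC_Quest_Test is an interactable test NPC in the quest system that talks to the player.
; On BeginPlay it hands its DialogueTree to its AIC_NPC AI controller.
; On Interact it yaws to face the player, plays a talk montage, then has the controller start the dialog without waiting for the montage to finish.
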(event EventBeginPlay
  ;[1 1 1] Set dialog tree
  (bind _asaic_npc (Utilities|Casting|CastToAIC_NPC (AI|GetAIController self)))
  (Variables|/Game/InventoryProject/Core/DialogSystem/AI/AIC_NPC.AIC_NPC_C|SetDialogueTree _asaic_npc (Variables|Default|GetDialogueTree)))

(event EventInteract
  (params (Interactor :type Actor%20Object%20Reference))
  ;[1 1 1] Rotate NPC towards player
  (Transformation|SetActorRotation (Math|Rotator|MakeRotator 0.0 0.0 (.yaw (Math|Rotator|FindLookatRotation (Transformation|GetActorLocation) (Transformation|GetActorLocation (Game|GetPlayerCharacter 0))))))
  (Animation|Montage|PlayMontage (Variables|Character|GetMesh) "/Game/InventoryProject/Characters/Test/Human/Male/Animations/AM_Human_Male_Talk.AM_Human_Male_Talk"
    (:then
      ;[1 1 1] Start dialog
      (bind _asaic_npc (Utilities|Casting|CastToAIC_NPC (AI|GetAIController self)))
      (Default|StartDialog _asaic_npc))))

(fn ConstructionScript)