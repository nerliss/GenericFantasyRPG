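; Explosive barrel quest object that reports player interaction to the quest system and plays an explosion effect.
; On Interact, it scans the quests in the player character's quest log and calls TargetInteracted on a quest for each uncompleted Interact-type objective.
; The explosion emitter attaches to the static mesh once per quest in the log, regardless of objective matches.
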(event EventBeginPlay)

(event Collision|EventActorBeginOverlap
  (params (OtherActor :type Actor%20Object%20Reference)))

(event EventTick
  (params (DeltaSeconds :type Float%20%28single-precision%29)))

(event EventInteract
  (params (Interactor :type Actor%20Object%20Reference))
  (bind _asbp_player_character (Utilities|Casting|CastToBP_PlayerCharacter Interactor))
  (for _array_element (Variables|/Game/InventoryProject/Core/QuestSystem/BP_Quest_LogComponent.BP_Quest_LogComponent_C|GetQuests (Variables|/Game/InventoryProject/Core/Characters/BP_PlayerCharacter.BP_PlayerCharacter_C|GetBP_Quest_LogComponent _asbp_player_character))
    ;[1 1 1] Check whether objective is of Interact type and hasn't been completed already
    (for _array_element_2 (Variables|/Game/InventoryProject/Core/QuestSystem/Quests/BP_Quest.BP_Quest_C|GetObjectives _array_element)
      (if (and (Utilities|Enum|Equal(Enum) (.Type (Utilities|Struct|BreakFObjective_Data _array_element_2)) "NewEnumerator1") (not (.bCompleted (Utilities|Struct|BreakFObjective_Data _array_element_2))))
        (Default|CallTargetInteracted _array_element self)))
    (Effects|SpawnEmitterAttached "/Game/StarterContent/Particles/P_Explosion.P_Explosion" (Variables|Default|GetStaticMesh) "None")))

(fn ConstructionScript)

(fn GetName
  (return ""))