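; Player character Blueprint that routes input to inventory, quest log, big map, minimap zoom, sprint and interaction, alongside several debug test keys.
; Tick traces from the camera to show HUD prompts for BPI_Interact actors, except during dialog.
; Landing speed prints placeholder fall-damage tiers or triggers Death, which plays a montage and disables input.
; Level-ups recalculate XP on unfinished quests, and the construction script disables Nanite.
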(event OnLevelGained(XPComp)
  ;[1 1 1] OnLevelGained event (pretty much heavy, need to rework once BP_Quest is written on C++)
  (bind _outactors (Actor|GetAllActorsOfClass "/Game/InventoryProject/Core/QuestSystem/Quests/BP_Quest.BP_Quest_C"))
  (for _array_element _outactors
    (if (not (Variables|/Game/InventoryProject/Core/QuestSystem/Quests/BP_Quest.BP_Quest_C|GetbCompleted _array_element))
      (Default|CalculateXP _array_element))))

(event EventOnLanded
  (params (Hit :type Hit%20Result%20Structure%20%28by%20ref%29))
  (bind _charactermovement (Variables|Character|GetCharacterMovement))
  (bind _velocity (Variables|/Script/Engine.MovementComponent|GetVelocity _charactermovement))
  (bind _returnvalue (* (.z _velocity) -1.0))
  ;[1 1 1] Fall damage (kinda)
  (if (Math|Float|InRange(Float) _returnvalue 1e+03 1.3e+03 true false)
    (Development|PrintString "1")
    (elif (Math|Float|InRange(Float) _returnvalue 1.3e+03 1.5e+03 true false)
      (Development|PrintString "2")
      (elif (Math|Float|InRange(Float) _returnvalue 1.5e+03 2e+03 true false)
        (Development|PrintString "3")
        (elif (> _returnvalue 2e+03)
          (CallFunction|Death))))))

(event EventTick
  (params (DeltaSeconds :type Float%20%28single-precision%29))
  ;[1 0 0] Tick
  (Utilities|FlowControl|Sequence
    (:then_0
      ;[1 1 1] Linetrace
      (if (not (Variables|Default|GetbInDialog))
        (bind _returnvalue (Class|RPGPlayerCharacter|LinetraceCamera (Variables|Default|GetTraceLength) false))
        (bind _hudref (Variables|Default|GetHUDRef)
          (:then
            (if (Utilities|DoesObjectImplementInterface _returnvalue "/Game/InventoryProject/Core/InventorySystem/BPI_Interact.BPI_Interact_C")
              (bind _name (Class|BPIInteract|GetName(Message) _returnvalue))
              (Default|DisplayMessage _hudref _returnvalue true _name)
              (else
                (Default|DisplayMessage _hudref 0 false))))
          (:else))
        (else
          (Default|DisplayMessage _hudref 0 false))))))

(event Input|ActionEvents|InputActionInteract
  (params (Key :type Key%20Structure :default "None"))
  ;[1 1 1] Interaction
  (:Pressed
    (Class|BPIInteract|Interact(Message) (Variables|Default|GetInteractActor) self)))

(event Input|ActionEvents|InputActionInventory
  (params (Key :type Key%20Structure :default "None"))
  ;[1 1 1] Open inventory
  (:Pressed
    (Default|InventoryToggle (Variables|Default|GetBP_InventoryComponent))))

(event Input|ActionEvents|InputActionMapZoomIn
  (params (Key :type Key%20Structure :default "None"))
  ;[1 1 1] Change map zoom
  (:Pressed
    (CallFunction|ChangeMapZoom 0.1)))

(event Input|ActionEvents|InputActionMapZoomOut
  (params (Key :type Key%20Structure :default "None"))
  ;[1 1 1] Change map zoom
  (:Pressed
    (CallFunction|ChangeMapZoom -0.1)))

(event Input|ActionEvents|InputActionToggleQuestLog
  (params (Key :type Key%20Structure :default "None"))
  ;[1 1 1] Toggle Quest Log
  (:Pressed
    (Default|ToggleQuestLog (Variables|Default|GetBP_Quest_LogComponent))))

(event Input|ActionEvents|InputActionToggleBigMap
  (params (Key :type Key%20Structure :default "None"))
  ;[1 1 1] Toggle Big Map
  (:Pressed
    (Utilities|FlowControl|FlipFlop
      (:A
        (bind _returnvalue (UserInterface|CreateWidget "/Game/InventoryProject/Core/Map/BigMap/WBP_BigMap.WBP_BigMap_C"))
        (UserInterface|Viewport|AddtoViewport _returnvalue 0))
      (:B
        (Widget|RemovefromParent _returnvalue)))))

(event Input|KeyboardEvents|RightBracket
  (params (Key :type Key%20Structure :default "None"))
  ;[1 0 0] TEST
  ;;[1 1 1] Query money
  (:Pressed
    (Default|MoneyQuery (Variables|Default|GetBP_InventoryComponent) (Utilities|Struct|MakeFMoney 8 96 53))))

(event Input|KeyboardEvents|G
  (params (Key :type Key%20Structure :default "None"))
  ;[1 0 0] TEST
  ;;[1 1 1] Add money
  (:Pressed
    (Default|MoneyAdd (Variables|Default|GetBP_InventoryComponent) 89653)))

(event Input|KeyboardEvents|1
  (params (Key :type Key%20Structure :default "None"))
  ;[1 0 0] TEST
  ;;[1 1 1] Questlog v2
  (:Pressed
    (bind _returnvalue (UserInterface|CreateWidget "/Game/InventoryProject/Core/QuestSystem/UI/WBP_Quest_Log_v2.WBP_Quest_Log_v2_C"))
    (UserInterface|Viewport|AddtoViewport _returnvalue 0)))

(event Input|KeyboardEvents|LeftShift
  (params (Key :type Key%20Structure :default "None"))
  (bind _charactermovement (Variables|Character|GetCharacterMovement))
  ;[1 1 1] Sprint
  (:Pressed
    (Variables|/Script/Engine.CharacterMovementComponent|SetMaxWalkSpeed _charactermovement 4.5e+03))
  (:Released
    (Variables|/Script/Engine.CharacterMovementComponent|SetMaxWalkSpeed _charactermovement 6e+02)))

(event Input|KeyboardEvents|P
  (params (Key :type Key%20Structure :default "None"))
  ;[1 0 0] TEST
  ;;[1 1 1] Death
  (:Pressed
    (CallFunction|Death)))

(event Input|KeyboardEvents|3
  (params (Key :type Key%20Structure :default "None"))
  ;[1 0 0] TEST
  ;;[1 1 1] TEST: Add xp
  (:Pressed
    (Class|RPGXPComponent|AddXP (Variables|Default|GetXPComp) 1e+02)))

(event Input|KeyboardEvents|4
  (params (Key :type Key%20Structure :default "None"))
  ;[1 0 0] TEST
  ;;[1 1 1] Get completed quests
  (:Pressed
    (Default|GetCompletedQuests (Variables|Default|GetBP_Quest_LogComponent))))

(event Input|KeyboardEvents|2
  (params (Key :type Key%20Structure :default "None"))
  ;[1 0 0] TEST
  ;;[1 1 1] Give Quest_002 to player as the game starts
  (:Pressed
    (bind _outactors (Actor|GetAllActorsOfClass "/Game/InventoryProject/Core/QuestSystem/Quests/BP_Quest_002.BP_Quest_002_C"))
    (bind _returnvalue (UserInterface|CreateWidget "/Game/InventoryProject/Core/QuestSystem/UI/WBP_Quest_DialogBox_Accept.WBP_Quest_DialogBox_Accept_C" 0 (Utilities|Array|Get(acopy) _outactors)))
    (bind _returnvalue_2 (Class|CanvasPanel|AddChildtoCanvas (Variables|/Game/InventoryProject/Core/UI/WBP_HUD.WBP_HUD_C|GetQuest_DialogBox_Holder (Variables|Default|GetHUDRef)) _returnvalue))
    (Class|CanvasPanelSlot|SetAutoSize _returnvalue_2 true)))

(fn ConstructionScript
  (Utilities|FlowControl|Sequence
    (:then_0
      ;[1 1 1] Disable Nanite if it is enabled
      (bind _returnvalue (Development|GetConsoleVariableIntValue "r.nanite"))
      (if (not (== _returnvalue 0))
        (Development|ExecuteConsoleCommand "r.nanite 0" 0)))))

(fn CameraLinetrace
  (params (LinetraceLength :type Float%20%28single-precision%29) (DrawDebugType :type EDrawDebugTrace%20Enum :default "None"))
  (bind _hudref (Variables|Default|GetHUDRef))
  (bind _cameracomp (Variables|Default|GetCameraComp))
  (bind _returnvalue (Transformation|GetWorldLocation _cameracomp))
  (bind (_outhit _returnvalue_2) (Collision|LineTraceByChannel _returnvalue (+ _returnvalue (* (Math|Vector|GetForwardVector _cameracomp) LinetraceLength)) "TraceTypeQuery2" true 0 DrawDebugType))
  (if _returnvalue_2
    (if (Utilities|DoesObjectImplementInterface (.HitActor (Collision|BreakHitResult _outhit)) "/Game/InventoryProject/Core/InventorySystem/BPI_Interact.BPI_Interact_C")
      (bind _output_get (Variables|Default|SetDEPRECATED_InteractActor (.HitActor (Collision|BreakHitResult _outhit))))
      (Default|DisplayMessage _hudref _output_get true)
      (return _output_get)
      (else
        _)))
  (bind _output_get_2 (Variables|Default|SetDEPRECATED_InteractActor 0))
  (Default|DisplayMessage _hudref 0 false)
  (return _output_get_2))

(fn Death
  (Animation|PlayAnimMontage "/Game/InventoryProject/Characters/Test/Human/Male/Animations/AM_Human_Male_Death.AM_Human_Male_Death" 1.0 "None")
  (Variables|Default|SetbDead true)
  (Audio|SpawnSound2D "/Game/InventoryProject/Sounds/Misc/A_Fart_01.A_Fart_01" 1.0 1.0 0.0 0)
  (Input|DisableInput (Game|GetPlayerController 0)))

(fn ChangeMapZoom
  (params (Amount :type Float%20%28single-precision%29))
  (bind _aspc_main (Utilities|Casting|CastToPC_Main (Game|GetPlayerController 0)))
  (Variables|/Game/InventoryProject/Core/Map/Minimap/WBP_Minimap.WBP_Minimap_C|SetZoom (Variables|/Game/InventoryProject/Core/UI/WBP_HUD.WBP_HUD_C|GetWBP_Minimap (Variables|/Game/InventoryProject/Core/PlayerControllers/PC_Main.PC_Main_C|GetHUD_Reference _aspc_main)) (Math|Float|Clamp(Float) (- (Variables|/Game/InventoryProject/Core/Map/Minimap/WBP_Minimap.WBP_Minimap_C|GetZoom (Variables|/Game/InventoryProject/Core/UI/WBP_HUD.WBP_HUD_C|GetWBP_Minimap (Variables|/Game/InventoryProject/Core/PlayerControllers/PC_Main.PC_Main_C|GetHUD_Reference _aspc_main))) Amount) 0.2)))