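; Enemy NPC that is killed through Interact, rewards the player, and can respawn in place.
; Death plays a montage, notifies every quest in the player's quest log, awards XP through the XP component and picks a random respawn delay.
; Interact also starts a delayed timer, while delete and respawn events toggle collision, mesh visibility and damageability instead of destroying the actor, with respawn clearing the death flags.
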(event Custom|Actor_Delete
  (bind _mesh (Variables|Character|GetMesh))
  ;[1 1 1] Delete/Respawn actor
  (Collision|SetCollisionEnabled _mesh "NoCollision")
  (Rendering|SetVisibility _mesh false false)
  (Variables|Default|SetbCanBeDamaged false)
  (Utilities|Time|SetTimerbyEvent (delegate Custom|Actor_Respawn) (Variables|Default|GetRespawnTime)))

(event Custom|Actor_Respawn
  (bind _mesh (Variables|Character|GetMesh))
  ;[1 1 1] Delete/Respawn actor
  (Variables|Default|SetbDead false)
  (Collision|SetCollisionEnabled _mesh "QueryAndPhysics")
  (Rendering|SetVisibility _mesh true false)
  (Variables|Default|SetbCanBeDamaged true)
  (Variables|Default|SetbDiedAlready false))

(event Custom|Death
  ;[1 1 1] Death. Awards XP, sets respawn timer, plays montage
  (if (and (not (Variables|Default|GetbDead)) (not (Variables|Default|GetbDiedAlready)))
    (Animation|Montage|PlayMontage (Variables|Character|GetMesh) (Variables|Default|GetAM_Death)
      (:then
        (Variables|Default|SetbDiedAlready true)
        (bind _asbp_player_character (Utilities|Casting|CastToBP_PlayerCharacter (Game|GetPlayerCharacter 0)))
        (for _array_element (Variables|/Game/InventoryProject/Core/QuestSystem/BP_Quest_LogComponent.BP_Quest_LogComponent_C|GetQuests (Variables|/Game/InventoryProject/Core/Characters/BP_PlayerCharacter.BP_PlayerCharacter_C|GetBP_Quest_LogComponent _asbp_player_character))
          (Default|CallEnemyKilled _array_element self))
        ;;[1 1 1] Award XP
        (bind _returnvalue (Class|RPGXPComponent|CalculateXPReward (Variables|/Script/InventoryProjectV3.RPGPlayerCharacter|GetXPComp _asbp_player_character) false 1.0))
        (Class|RPGXPComponent|AddXP (Variables|/Script/InventoryProjectV3.RPGPlayerCharacter|GetXPComp _asbp_player_character) _returnvalue)
        (Variables|Default|SetRespawnTime (Math|Random|RandomFloatinRange 3e+01 6e+01)))
      (:OnBlendOut
        (Variables|Default|SetbDead true)))))

(event EventInteract
  (params (Interactor :type Actor%20Object%20Reference))
  (CallFunction|Death)
  (Utilities|Time|SetTimerbyEvent (EventDispatchers|CreateEvent :!event Custom|Actor_Delete) 15.0))

(fn ConstructionScript
  (|CallParentFunction))