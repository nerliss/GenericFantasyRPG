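; Base NPC Blueprint that the player can talk to through the dialog system.
; On BeginPlay it passes its dialogue tree to the AIC_NPC controller and caches the player.
; Interacting while not falling turns the NPC toward the player, plays a talk montage and greeting, starts the controller's dialog, and notifies quests with unfinished interact objectives.
; EndDialog plays a farewell sound; death and quest-marker logic is present but unconnected.
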(event Custom|EndDialog
  ;[1 1 1] Mostly used for cosmetic and\or customizable things
  (Audio|SpawnSound2D (Variables|Default|GetSound_Farewell) 1.0 1.0 0.0 0))

(event EventBeginPlay
  (Utilities|FlowControl|Sequence
    (:then_0
      ;[1 1 1] Set dialog tree
      (bind _asaic_npc (Utilities|Casting|CastToAIC_NPC (AI|GetAIController self)))
      (Variables|/Game/InventoryProject/Core/DialogSystem/AI/AIC_NPC.AIC_NPC_C|SetDialogueTree _asaic_npc (Variables|Default|GetDialogueTree))
      ;[1 1 1] Set player reference
      (bind _asbp_player_character (Utilities|Casting|CastToBP_PlayerCharacter (Game|GetPlayerCharacter 0)))
      (Variables|Default|SetPlayerRef _asbp_player_character))))

(event EventInteract
  (params (Interactor :type Actor%20Object%20Reference))
  (if (not (AI|Components|NavMovement|IsFalling (Variables|/Script/Engine.Character|GetCharacterMovement (.AsBP%20Player%20Character (Utilities|Casting|CastToBP_PlayerCharacter Interactor)))))
    ;[1 1 1] Rotate NPC towards player
    (Transformation|SetActorRotation (Math|Rotator|MakeRotator 0.0 0.0 (.yaw (Math|Rotator|FindLookatRotation (Transformation|GetActorLocation) (Transformation|GetActorLocation (Game|GetPlayerCharacter 0))))))
    ;[1 1 1] Play montage and sound for greetings
    (Animation|Montage|PlayMontage (Variables|Character|GetMesh) (Variables|Default|GetAM_Talk)
      (:then
        (Audio|SpawnSoundatLocation (Variables|Default|GetSound_Greetings) (Transformation|GetActorLocation) "0, 0, 0" 1.0 1.0 0.0 "/Game/InventoryProject/Sounds/ATT_Base.ATT_Base" 0)
        ;[1 1 1] Start dialog
        (bind _asaic_npc (Utilities|Casting|CastToAIC_NPC (AI|GetAIController self)))
        (Default|StartDialog _asaic_npc)
        ;[1 1 1] Interaction objective completion call. Perhaps should be implemented elsewhere since we have a complete dialog system
        (for _array_element (Variables|/Game/InventoryProject/Core/QuestSystem/BP_Quest_LogComponent.BP_Quest_LogComponent_C|GetQuests (Variables|/Game/InventoryProject/Core/Characters/BP_PlayerCharacter.BP_PlayerCharacter_C|GetBP_Quest_LogComponent (Variables|Default|GetPlayerRef)))
          ;;[1 1 1] Check whether objective is of Interact type and hasn't been completed already
          (for _array_element_2 (Variables|/Game/InventoryProject/Core/QuestSystem/Quests/BP_Quest.BP_Quest_C|GetObjectives _array_element)
            (if (and (Utilities|Enum|Equal(Enum) (.Type (Utilities|Struct|BreakFObjective_Data _array_element_2)) "NewEnumerator1") (not (.bCompleted (Utilities|Struct|BreakFObjective_Data _array_element_2))))
              (Default|CallTargetInteracted _array_element self))))))))

(event Collision|EventHit
  (params (MyComp :type Primitive%20Component%20Object%20Reference) (Other :type Actor%20Object%20Reference) (OtherComp :type Primitive%20Component%20Object%20Reference) (bSelfMoved :type Boolean) (HitLocation :type Vector :default "0, 0, 0") (HitNormal :type Vector :default "0, 0, 0") (NormalImpulse :type Vector :default "0, 0, 0") (Hit :type Hit%20Result%20Structure%20%28by%20ref%29)))

(fn ConstructionScript)

(fn GetName
  (return (Variables|Default|GetName)))