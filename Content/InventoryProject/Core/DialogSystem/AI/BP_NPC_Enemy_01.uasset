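; BP_NPC_Enemy_01 is an enemy NPC whose Interact event acts as a test death that credits quests.
; While not Dead, interacting plays a death montage and immediately calls EnemyKilled on every quest in the player's BPQuestLogComponent, passing itself.
; Dead is set only when the montage blends out, so interactions before then can trigger the credit again.
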(event EventBeginPlay
  (|CallParentFunction) ; This node is disabled and will not be called.\nDrag off pins to build functionality.
)

(event Collision|EventActorBeginOverlap
  (params (OtherActor :type Actor%20Object%20Reference)))

(event EventTick
  (params (DeltaSeconds :type Float%20%28single-precision%29)))

(event EventInteract
  (params (Interactor :type Actor%20Object%20Reference))
  ;[1 1 1] TEST: Death. Give credit to quest if there is one
  (if (not (Variables|Default|GetbDead))
    (Animation|Montage|PlayMontage (Variables|Character|GetMesh) "/Game/InventoryProject/Characters/Test/Broken/Animations/AM_Broken_Death.AM_Broken_Death"
      (:then
        (bind _asbp_player_character (Utilities|Casting|CastToBP_PlayerCharacter (Game|GetPlayerCharacter 0)))
        (for _array_element (Variables|/Game/InventoryProject/Core/QuestSystem/BP_Quest_LogComponent.BP_Quest_LogComponent_C|GetQuests (Variables|/Game/InventoryProject/Core/Characters/BP_PlayerCharacter.BP_PlayerCharacter_C|GetBP_Quest_LogComponent _asbp_player_character))
          (Default|CallEnemyKilled _array_element self)
          (Development|PrintString "Target killed!")))
      (:OnBlendOut
        (Variables|Default|SetbDead true)))))

(fn ConstructionScript
  (|CallParentFunction))