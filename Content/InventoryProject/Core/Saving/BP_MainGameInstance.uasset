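; Game instance that owns the save game, persisting player transform and XP component progress (XP, level, skill points).
; Init loads the existing save slot and starts a looping five-second Autosave timer, or creates a fresh save object without starting that timer.
; Save, load and clear functions move data between the player character and the slot.
; Inventory save and load nodes exist but are disconnected.
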(event EventInit
  ;[1 1 1] Setup save game file
  (bind _returnvalue (SaveGame|DoesSaveGameExist (Variables|Default|GetSaveSlotName)))
  (if _returnvalue
    (bind _returnvalue_2 (SaveGame|LoadGamefromSlot (Variables|Default|GetSaveSlotName)))
    (bind _asbp_save_game_object (Utilities|Casting|CastToBP_SaveGameObject _returnvalue_2))
    (Variables|Default|SetSaveGameObjectRef _asbp_save_game_object)
    (Utilities|Time|SetTimerbyFunctionName 0 "Autosave" 5.0 true)
    (else
      (bind _returnvalue_3 (SaveGame|CreateSaveGameObject "/Game/InventoryProject/Core/Saving/BP_SaveGameObject.BP_SaveGameObject_C"))
      (Variables|Default|SetSaveGameObjectRef _returnvalue_3))))

(fn SaveDataPlayer
  (Utilities|FlowControl|Sequence
    (:then_0
      (bind _asbp_player_character (Utilities|Casting|CastToBP_PlayerCharacter (Game|GetPlayerCharacter 0)))
      (bind _output_get (LocalVariables|SetPlayerRef _asbp_player_character))
      (Variables|/Game/InventoryProject/Core/Saving/BP_SaveGameObject.BP_SaveGameObject_C|SetData_Player (Variables|Default|GetSaveGameObjectRef) (Utilities|Struct|MakeFSave_Player (Transformation|GetActorTransform _output_get) (Variables|/Script/InventoryProjectV3.RPGXP_Component|GetXP_Current (Variables|/Script/InventoryProjectV3.RPGPlayerCharacter|GetXPComp _output_get)) (Variables|/Script/InventoryProjectV3.RPGXP_Component|GetXP_Buffer (Variables|/Script/InventoryProjectV3.RPGPlayerCharacter|GetXPComp _output_get)) (Variables|/Script/InventoryProjectV3.RPGXP_Component|GetXP_Current_Max (Variables|/Script/InventoryProjectV3.RPGPlayerCharacter|GetXPComp _output_get)) (Variables|/Script/InventoryProjectV3.RPGXP_Component|GetLevel_Current (Variables|/Script/InventoryProjectV3.RPGPlayerCharacter|GetXPComp _output_get)) (Variables|/Script/InventoryProjectV3.RPGXP_Component|GetSkillPoints (Variables|/Script/InventoryProjectV3.RPGPlayerCharacter|GetXPComp _output_get)))))
    (:then_1
      (SaveGame|SaveGametoSlot (Variables|Default|GetSaveGameObjectRef) (Variables|Default|GetSaveSlotName)))))

(fn LoadDataPlayer
  (bind _savegameobjectref (Variables|Default|GetSaveGameObjectRef))
  (bind _data_player (Variables|/Game/InventoryProject/Core/Saving/BP_SaveGameObject.BP_SaveGameObject_C|GetData_Player _savegameobjectref))
  (bind _asbp_player_character (Utilities|Casting|CastToBP_PlayerCharacter (Game|GetPlayerCharacter 0)))
  (bind _output_get (LocalVariables|SetPlayerRef _asbp_player_character))
  (Variables|/Script/InventoryProjectV3.RPGXP_Component|SetXP_Current (Variables|/Script/InventoryProjectV3.RPGPlayerCharacter|GetXPComp _output_get) (.xp_current _data_player))
  (Variables|/Script/InventoryProjectV3.RPGXP_Component|SetXP_Buffer (Variables|/Script/InventoryProjectV3.RPGPlayerCharacter|GetXPComp _output_get) (.xp_buffer _data_player))
  (Variables|/Script/InventoryProjectV3.RPGXP_Component|SetXP_Current_Max (Variables|/Script/InventoryProjectV3.RPGPlayerCharacter|GetXPComp _output_get) (.xp_current_max _data_player))
  (Variables|/Script/InventoryProjectV3.RPGXP_Component|SetLevel_Current (Variables|/Script/InventoryProjectV3.RPGPlayerCharacter|GetXPComp _output_get) (.level_current _data_player))
  (Variables|/Script/InventoryProjectV3.RPGXP_Component|SetSkillPoints (Variables|/Script/InventoryProjectV3.RPGPlayerCharacter|GetXPComp _output_get) (.skillpoints _data_player))
  (Transformation|SetActorTransform _output_get (.transform _data_player)))

(fn ClearSaveData
  (SaveGame|DeleteGameinSlot (Variables|Default|GetSaveSlotName)))

(fn Autosave
  (CallFunction|SaveDataPlayer))