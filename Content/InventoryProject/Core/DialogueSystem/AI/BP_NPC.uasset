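; BP_NPC is a human NPC that greets the player on interaction and dies when hit by a projectile.
; Interact turns it toward the player and plays a talk montage and greeting, then a five-second retriggerable delay restores a fixed yaw and plays a farewell.
; A hit from a FirstPersonProjectile plays a death montage and sound and sets Dead, which nothing in these graphs reads.
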(event Collision|EventHit
  (params (MyComp :type Primitive%20Component%20Object%20Reference) (Other :type Actor%20Object%20Reference) (OtherComp :type Primitive%20Component%20Object%20Reference) (bSelfMoved :type Boolean) (HitLocation :type Vector :default "0, 0, 0") (HitNormal :type Vector :default "0, 0, 0") (NormalImpulse :type Vector :default "0, 0, 0") (Hit :type Hit%20Result%20Structure%20%28by%20ref%29))
  (Utilities|Casting|CastToFirstPersonProjectile Other)
  (Animation|Montage|PlayMontage (Variables|Character|GetMesh) "/Game/InventoryProject/Characters/Test/Human/Male/Animations/AM_Human_Male_Death.AM_Human_Male_Death"
    (:then
      (Audio|SpawnSoundatLocation "/Game/InventoryProject/Sounds/Characters/Test/Kingpin_-_Death_Cue.Kingpin_-_Death_Cue" (Transformation|GetActorLocation) "0, 0, 0" 1.0 1.0 0.0 "/Game/InventoryProject/Sounds/ATT_Base.ATT_Base" 0)
      (Variables|Default|SetbDead true))))

(event EventInteract
  (params (Interactor :type Actor%20Object%20Reference))
  ;[1 1 1] Rotate NPC towards player
  (Transformation|SetActorRotation (Math|Rotator|MakeRotator 0.0 0.0 (.yaw (Math|Rotator|FindLookatRotation (Transformation|GetActorLocation) (Transformation|GetActorLocation (Game|GetPlayerCharacter 0))))))
  (Animation|Montage|PlayMontage (Variables|Character|GetMesh) "/Game/InventoryProject/Characters/Test/Human/Male/Animations/AM_Human_Male_Talk.AM_Human_Male_Talk"
    (:then
      (Audio|SpawnSoundatLocation "/Game/InventoryProject/Sounds/Characters/Test/Kingpin_-_Greetings_Cue.Kingpin_-_Greetings_Cue" (Transformation|GetActorLocation) "0, 0, 0" 1.0 1.0 0.0 "/Game/InventoryProject/Sounds/ATT_Base.ATT_Base" 0)
      (Utilities|FlowControl|RetriggerableDelay 5.0)
      (Transformation|SetActorRotation (Math|Rotator|MakeRotator 0.0 0.0 9e+01))
      (Audio|SpawnSoundatLocation "/Game/InventoryProject/Sounds/Characters/Test/Kingpin_-_Farewell_Cue.Kingpin_-_Farewell_Cue" (Transformation|GetActorLocation) "0, 0, 0" 1.0 1.0 0.0 "/Game/InventoryProject/Sounds/ATT_Base.ATT_Base" 0))))

(fn ConstructionScript)