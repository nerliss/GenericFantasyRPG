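; Skill system component that tracks unlocked skills and toggles the skill window UI.
; Skills live in a map of row name to tier: adding inserts at tier 1 or increments it, and queries return the tier.
; The window is created lazily on the PC_Main HUD canvas, then shown or hidden.
; Toggling switches input mode and mouse cursor, and showing the window calls SetSkillWindowVisible.
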(event EventBeginPlay)

(event EventTick
  (params (DeltaSeconds :type Float%20%28single-precision%29)))

(fn SkillAdd
  (params (Row_name :type String))
  (bind _skill_unlocked (Variables|Default|GetSkill_Unlocked))
  (bind (_value _returnvalue) (Utilities|Map|Find _skill_unlocked Row_name))
  (if _returnvalue ; Check if we already have a skill with that name
    (Utilities|Map|Add _skill_unlocked Row_name (+ _value 1))
    (Development|PrintString (Utilities|String|Append Row_name " was successfully updated!") true true "(R=0.000000,G=0.190395,B=1.000000,A=1.000000)")
    (else
      (Utilities|Map|Add _skill_unlocked Row_name 1)
      (Development|PrintString (Utilities|String|Append Row_name " was successfully added!") true true "(R=0.293042,G=1.000000,B=0.000000,A=1.000000)")))
  (return true))

(fn SkillQuery
  (params (Row%20name :type String))
  (bind _skill_unlocked (Variables|Default|GetSkill_Unlocked))
  (bind (_value _returnvalue) (Utilities|Map|Find _skill_unlocked Row%20name))
  (if _returnvalue ; Check if we have a given skill
    (return true _value)
    (else
      (return false 0))))

(fn ToggleSkillWindow
  (bind _returnvalue (Game|GetPlayerController 0))
  (bind _returnvalue_2 (Game|GetPlayerController 0))
  (Variables|Default|GetSkillWindow_Ref ; Check if reference is valid and if yes - switch visibily, otherwise create reference. It is made that way because the skill system doesn't take all the information from DT and obviously doesn't allow to edit it as well. So I had to do this this way. IT JUST DOESN'T WORK THE DEFAULT REFERENCE WAY
    (:then
      (if (Variables|Default|GetbVisible)
        (Widget|SetVisibility (Variables|Default|GetSkillWindow_Ref) "Hidden")
        (Input|SetInputModeGameOnly _returnvalue_2)
        (Variables|/Script/Engine.PlayerController|SetbShowMouseCursor _returnvalue_2 false)
        (Variables|Default|SetbVisible false)
        (else
          (Widget|SetVisibility (Variables|Default|GetSkillWindow_Ref) "Visible")
          (Input|SetInputModeUIOnly _returnvalue_2 (Variables|Default|GetSkillWindow_Ref) "LockAlways")
          (Variables|/Script/Engine.PlayerController|SetbShowMouseCursor _returnvalue_2 true)
          (Variables|Default|SetbVisible true)
          (Default|CallSetSkillWindowVisible))))
    (:else
      (bind _returnvalue_3 (UserInterface|CreateWidget "/Game/InventoryProject/Core/SkillSystem/UI/WBP_Skill_Window.WBP_Skill_Window_C"))
      (bind _output_get (Variables|Default|SetSkillWindow_Ref _returnvalue_3))
      (bind _aspc_main (Utilities|Casting|CastToPC_Main (Game|GetPlayerController 0)))
      (Variables|/Game/InventoryProject/Core/UI/WBP_HUD.WBP_HUD_C|SetSkillWindowRef (Variables|/Game/InventoryProject/Core/PlayerControllers/PC_Main.PC_Main_C|GetHUD_Reference _aspc_main) _output_get)
      (bind _returnvalue_4 (Class|CanvasPanel|AddChildtoCanvas (Variables|/Game/InventoryProject/Core/UI/WBP_HUD.WBP_HUD_C|GetHUDCanvas (Variables|/Game/InventoryProject/Core/PlayerControllers/PC_Main.PC_Main_C|GetHUD_Reference _aspc_main)) _output_get))
      ;[1 1 1] Set position of the window
      (Class|CanvasPanelSlot|SetAutoSize _returnvalue_4 true)
      (Class|CanvasPanelSlot|SetAlignment _returnvalue_4 (LocalVariables|GetAlignment))
      (Class|CanvasPanelSlot|SetAnchors _returnvalue_4 (LocalVariables|GetAnchors))
      (Input|SetInputModeUIOnly _returnvalue _output_get "LockAlways")
      (Variables|/Script/Engine.PlayerController|SetbShowMouseCursor _returnvalue true)
      (Variables|Default|SetbVisible true)
      (Default|CallSetSkillWindowVisible))))