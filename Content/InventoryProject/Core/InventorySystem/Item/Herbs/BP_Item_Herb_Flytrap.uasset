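; Flytrap herb item Blueprint that the player gathers into the inventory and can use for experience.
; Interacting adds a random stack of several units to the interactor's inventory.
; Using it awards the player character a small scaled XP reward through its XP component, then runs the parent item's use logic.
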(event EventBeginPlay)

(event Collision|EventActorBeginOverlap
  (params (OtherActor :type Actor%20Object%20Reference)))

(event EventTick
  (params (DeltaSeconds :type Float%20%28single-precision%29)))

(event EventInteract
  (params (Interactor :type Actor%20Object%20Reference))
  (CallFunction|AddtoInventory Interactor (Math|Random|RandomIntegerinRange 3 7)))

(fn ConstructionScript
  (|CallParentFunction))

(fn ItemUse
  (bind _returnvalue (Game|GetPlayerCharacter 0))
  (bind _asbp_player_character (Utilities|Casting|CastToBP_PlayerCharacter _returnvalue))
  (bind _xpcomp (Variables|/Script/InventoryProjectV3.RPGPlayerCharacter|GetXPComp _asbp_player_character))
  (bind _returnvalue_2 (Class|RPGXPComponent|CalculateXPReward _xpcomp false 0.1))
  (Class|RPGXPComponent|AddXP _xpcomp _returnvalue_2)
  (bind _success (|CallParentFunction))
  (return _success))