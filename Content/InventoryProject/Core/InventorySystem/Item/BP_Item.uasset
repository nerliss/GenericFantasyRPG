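; BP_Item is a pickup actor that, when interacted with, adds one of its FItem to the interactor's inventory component and destroys itself on success.
; Quest items are only picked up when an objective in the player's quest log targets the same item class.
; A successful pickup notifies quests with uncompleted collect-type objectives through CallItemCollected, while a failed add prints a message.
; UseItem is a stub that returns true.
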(event Custom|UpdateObjectives
  (bind _asbp_player_character (Utilities|Casting|CastToBP_PlayerCharacter (Game|GetPlayerCharacter 0)))
  (for _array_element (Variables|/Game/InventoryProject/Core/QuestSystem/BP_Quest_LogComponent.BP_Quest_LogComponent_C|GetQuests (Variables|/Game/InventoryProject/Core/Characters/BP_PlayerCharacter.BP_PlayerCharacter_C|GetBP_Quest_LogComponent _asbp_player_character))
    ;[1 1 1] Check whether objective is of Collect type and hasn't been completed already
    (for _array_element_2 (Variables|/Game/InventoryProject/Core/QuestSystem/Quests/BP_Quest.BP_Quest_C|GetObjectives _array_element)
      (if (and (Utilities|Enum|Equal(Enum) (.Type (Utilities|Struct|BreakFObjective_Data _array_element_2)) "NewEnumerator2") (not (.bCompleted (Utilities|Struct|BreakFObjective_Data _array_element_2))))
        (Default|CallItemCollected _array_element self)))))

(event EventInteract
  (params (Interactor :type Actor%20Object%20Reference))
  (if (.bquestitem (Variables|Default|GetFItem))
    ;[1 1 1] If an item is a quest realted (Quest Item) and player has this quest - add to inventory
    (bind _asbp_player_character (Utilities|Casting|CastToBP_PlayerCharacter (Game|GetPlayerCharacter 0)))
    (for _array_element (Variables|/Game/InventoryProject/Core/QuestSystem/BP_Quest_LogComponent.BP_Quest_LogComponent_C|GetQuests (Variables|/Game/InventoryProject/Core/Characters/BP_PlayerCharacter.BP_PlayerCharacter_C|GetBP_Quest_LogComponent _asbp_player_character))
      (for _array_element_2 (Variables|/Game/InventoryProject/Core/QuestSystem/Quests/BP_Quest.BP_Quest_C|GetObjectives _array_element)
        (if (== (Utilities|GetClass (.Target (Utilities|Struct|BreakFObjective_Data _array_element_2))) (Utilities|GetClass self))
          (CallFunction|AddtoInventory Interactor 1))))
    (else
      (CallFunction|AddtoInventory Interactor 1))))

(fn ConstructionScript)

(fn AddtoInventory
  (params (Interactor :type Actor%20Object%20Reference) (QuantityOfItemsToAdd :type Integer))
  (bind _fitem (Variables|Default|GetFItem))
  (bind _fslot (Utilities|Struct|MakeFSlot _fitem QuantityOfItemsToAdd))
  (bind _bsuccess (Default|AddtoInventory (Actor|GetComponentbyClass Interactor "/Game/InventoryProject/Core/InventorySystem/BP_InventoryComponent.BP_InventoryComponent_C") _fslot))
  (if _bsuccess
    (CallFunction|UpdateObjectives)
    (Actor|DestroyActor)
    (else
      (Development|PrintString (Utilities|String|Append (Utilities|String|ToString(Text) (.name (.FItem (Utilities|Struct|BreakFSlot _fslot)))) " failed to add to inventory")))))

(fn UseItem
  (return true))