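; BP_Container is an interactable container, such as a chest, that holds items in its own inventory component.
; On BeginPlay it copies its Items array into the component's Inventory, slot by slot at matching indices.
; Interact toggles that inventory when the interactor is a BP_FirstPersonCharacter, printing a debug message on success or failed cast.
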(event EventInteract
  (params (Interactor :type Actor%20Object%20Reference))
  (Utilities|Casting|CastToBP_FirstPersonCharacter Interactor
    (:then
      (Default|ToggleInventory (Variables|Default|GetBP_InventoryComponent))
      (Development|PrintString "The chest was successfully opened!"))
    (:CastFailed
      (Development|PrintString "Cast to chest failed"))))

(event EventBeginPlay
  (for (_array_element _array_index) (Variables|Default|GetItems)
    (Utilities|Array|SetArrayElem (Variables|/Game/InventoryProject/Core/InventorySystem/BP_InventoryComponent.BP_InventoryComponent_C|GetInventory (Variables|Default|GetBP_InventoryComponent)) _array_index _array_element)))

(fn ConstructionScript)