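; Inventory component that stores items in a fixed-size slot array and toggles the inventory window on the HUD canvas, switching input mode and cursor.
; PrepareInventory sizes the array and refills item data from class defaults on BeginPlay and window opening.
; AddToInventory tops up partial stacks of stackable items, recursing on overflow, or creates stacks in empty slots.
; It always returns true, with no full-inventory check.
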(event EventBeginPlay
  (CallFunction|PrepareInventory))

(fn ToggleInventory
  (bind _returnvalue (Game|GetPlayerController 0))
  (bind _returnvalue_2 (Game|GetPlayerController 0))
  (bind _inventorywindow_ref (Variables|Default|GetInventoryWindow_Ref)
    (:then
      (Widget|RemovefromParent _inventorywindow_ref)
      (Variables|Default|SetInventoryWindow_Ref 0)
      (Input|SetInputModeGameOnly _returnvalue_2)
      (Variables|/Script/Engine.PlayerController|SetbShowMouseCursor _returnvalue_2 false))
    (:else
      (CallFunction|PrepareInventory)
      (bind _returnvalue_3 (UserInterface|CreateWidget "/Game/InventoryProject/Core/InventorySystem/UI/WBP_Inventory_Window.WBP_Inventory_Window_C" 0 self))
      (bind _output_get (Variables|Default|SetInventoryWindow_Ref _returnvalue_3))
      (bind _aspc_main (Utilities|Casting|CastToPC_Main (Game|GetPlayerController 0)))
      (bind _returnvalue_4 (Class|CanvasPanel|AddChildtoCanvas (Variables|/Game/InventoryProject/Core/InventorySystem/UI/WBP_HUD.WBP_HUD_C|GetHUDCanvas (Variables|/Game/InventoryProject/Core/PlayerControllers/PC_Main.PC_Main_C|GetHUD_Reference _aspc_main)) _output_get))
      ;[1 1 1] Set position of the window
      (Class|CanvasPanelSlot|SetAutoSize _returnvalue_4 true)
      (Class|CanvasPanelSlot|SetAlignment _returnvalue_4 (Variables|Default|GetAlignment))
      (Class|CanvasPanelSlot|SetAnchors _returnvalue_4 (Variables|Default|GetAnchors))
      (Input|SetInputModeUIOnly _returnvalue _output_get "LockAlways")
      (Variables|/Script/Engine.PlayerController|SetbShowMouseCursor _returnvalue true))))

(fn AddtoInventory
  (params (ContentToAdd :type F%20Slot%20Structure))
  (bind (_fitem _quantity) (Utilities|Struct|BreakFSlot ContentToAdd))
  (bind _returnvalue (Utilities|String|ToString(Text) (.name _fitem)))
  (bind _returnvalue_2 (Utilities|String|ToString(Integer) _quantity))
  (if (.bstackable _fitem)
    (bind _stackslotindex (Utilities|HasPartialStack ContentToAdd)
      (:True
        (CallFunction|AddtoStack ContentToAdd _stackslotindex)
        (Development|PrintString (Utilities|String|Append "Successfully added item to already existing stack: " _returnvalue ". Items added: " _returnvalue_2) true true "(R=0.101204,G=1.000000,B=0.134408,A=1.000000)" 4.0))
      (:False
        (CallFunction|CreateStack ContentToAdd :!label _label)
        (Development|PrintString (Utilities|String|Append "Stack successfully created and item added: " _returnvalue ". Items added: " _returnvalue_2) true true "(R=0.545177,G=0.531250,B=1.000000,A=1.000000)" 4.0)))
    (else
      (goto _label)))
  (return true))

(fn PrepareInventory
  (bind _inventory (Variables|Default|GetInventory))
  (Utilities|Array|Resize _inventory (Variables|Default|GetSlots_Number))
  (for (_array_element _array_index) _inventory
    (if (!= (.Class (Utilities|Struct|BreakFItem (.fitem _array_element))) 0)
      (Utilities|Array|SetArrayElem _inventory _array_index (Utilities|Struct|MakeFSlot (Utilities|GetClassDefaults (.Class (Utilities|Struct|BreakFItem (.fitem _array_element)))) (.quantity _array_element))))))

(fn CreateStack
  (params (ContentToAdd :type F%20Slot%20Structure))
  (bind _inventory (Variables|Default|GetInventory))
  (Utilities|Array|SetArrayElem _inventory (Utilities|Array|FindItem _inventory (Utilities|Struct|MakeFSlot "(Name_2_2F6061E44AF3110F9E97A39AFF82CF4A=NSLOCTEXT(\"[5AA1FCF64387F5C2F9ED7C8CF0307F11]\", \"5E2462AF42D218EE2EE981A727352EA6\", \"PH_Name\"),Description_11_96A16BE14CCDF78EB8ACCA849DA532C9=NSLOCTEXT(\"[5AA1FCF64387F5C2F9ED7C8CF0307F11]\", \"D21895594CF85F30602CCFAC2F262704\", \"PH_Desc\"),bStackable_5_1490E9B8434DBA39FB4AAE9A50F6D636=True,bConsumable_14_B709E8E24A198A4F222A3A80E155A806=False,Thumbnail_8_8196840D4E4DDF941CDE63ABB0A59B0A=None,MaxStackSize_17_99ED06AB45A69C67F75E028E71864490=20,Durability_20_082FA4C94375127EAEEF8AA9C7CD6B2C=0.000000,Class_23_C84069DE45D26748B6BC7C97CD5DE955=None)")) ContentToAdd))

(fn AddtoStack
  (params (FSlot :type F%20Slot%20Structure) (SlotIndex :type Integer))
  (bind (_fitem _quantity) (Utilities|Struct|BreakFSlot FSlot))
  (bind _inventory (Variables|Default|GetInventory))
  (bind _maxstacksize (Utilities|Struct|BreakFItem _fitem))
  (bind _output (Utilities|Array|Get(acopy) _inventory SlotIndex))
  (bind (_fitem_2 _quantity_2) (Utilities|Struct|BreakFSlot _output))
  (bind (_fitem_3 _quantity_3) (Utilities|Struct|BreakFSlot _output))
  ;[1 1 1] IDK IT JUST WORKS
  (bind _output_get (LocalVariables|SetCurrentQuantity _quantity_2))
  (if (> (+ _output_get _quantity) (.maxstacksize _fitem_2)) ; Check whether new quantity value is bigger than max stack size and if yes - add to existing and create a new stack
    (Utilities|Array|SetArrayElem _inventory SlotIndex (Utilities|Struct|MakeFSlot _fitem _maxstacksize))
    (CallFunction|AddtoInventory (Utilities|Struct|MakeFSlot _fitem (- _quantity (- _maxstacksize _output_get))))
    (else
      (Utilities|Array|SetArrayElem _inventory SlotIndex (Utilities|Struct|MakeFSlot _fitem_3 (+ _quantity _quantity_3)))))
  (return))