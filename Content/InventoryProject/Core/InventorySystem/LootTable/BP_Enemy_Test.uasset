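; Test enemy actor for the inventory project's loot system that dies from a projectile hit and can then be looted.
; The first FirstPersonProjectile hit passes a DoOnce, marks it Dead, reveals HealthStatus and, as a test, swaps the player's minimap image through the HUD.
; Interact drops loot from BPLootTable and toggles BPInventoryComponent when dead, otherwise it prints a placeholder greeting.
; GetName exposes its Name.
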(event EventBeginPlay)

(event Collision|EventHit
  (params (MyComp :type Primitive%20Component%20Object%20Reference) (Other :type Actor%20Object%20Reference) (OtherComp :type Primitive%20Component%20Object%20Reference) (bSelfMoved :type Boolean) (HitLocation :type Vector :default "0, 0, 0") (HitNormal :type Vector :default "0, 0, 0") (NormalImpulse :type Vector :default "0, 0, 0") (Hit :type Hit%20Result%20Structure%20%28by%20ref%29))
  ;[1 1 1] Test functionality - add item to player's inventory upon hit from projectile
  (Utilities|Casting|CastToFirstPersonProjectile Other)
  (Utilities|FlowControl|DoOnce false
    (:Completed
      (Variables|Default|SetbDead true)
      (Development|SetHiddeninGame (Variables|Default|GetHealthStatus) false false)
      ;[1 1 1] Set new map texture - TEST
      (bind _aspc_main (Utilities|Casting|CastToPC_Main (Game|GetPlayerController 0)))
      (Default|UpdateMapImage (Variables|/Game/InventoryProject/Core/UI/WBP_HUD.WBP_HUD_C|GetWBP_Minimap (Variables|/Game/InventoryProject/Core/PlayerControllers/PC_Main.PC_Main_C|GetHUD_Reference _aspc_main)) (Variables|Default|GetMap_Test)))))

(event EventInteract
  (params (Interactor :type Actor%20Object%20Reference))
  (if (Variables|Default|GetbDead)
    (Default|DropLoot (Variables|Default|GetBP_LootTable))
    (Default|InventoryToggle (Variables|Default|GetBP_InventoryComponent))
    (else
      (Development|PrintString "Yo wassup"))))

(fn ConstructionScript)

(fn GetName
  (return (Variables|Default|GetName)))