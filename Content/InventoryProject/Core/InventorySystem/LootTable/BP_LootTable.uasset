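; BP_LootTable is a weighted loot table that fills a dead test enemy's inventory with a randomly chosen item.
; DropLoot totals the LootTable weights, then ChooseLoot picks a key by subtracting weights from a random roll.
; It adds a fixed quantity of that item's class defaults to the first dead BP_Enemy_Test found among all such actors.
; An unconnected branch would give the item to the player instead.
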(event Custom|DropLoot
  (bind _totalsum (CallFunction|CalculateSum))
  (Variables|Default|SetValueSum _totalsum)
  (bind _loot (CallFunction|ChooseLoot))
  (bind _outactors (Actor|GetAllActorsOfClass "/Game/InventoryProject/Core/InventorySystem/LootTable/BP_Enemy_Test.BP_Enemy_Test_C"))
  (bind _array_element (Utilities|Array|ForEachLoopwithBreak _outactors :!label _label)
    (:LoopBody
      (if (Variables|/Game/InventoryProject/Core/InventorySystem/LootTable/BP_Enemy_Test.BP_Enemy_Test_C|GetbDead _array_element)
        (Default|AddtoInventory (Variables|/Game/InventoryProject/Core/InventorySystem/LootTable/BP_Enemy_Test.BP_Enemy_Test_C|GetBP_InventoryComponent _array_element) (Utilities|Struct|MakeFSlot (Utilities|GetClassDefaults _loot) 3))
        (goto _label Break)))))

(fn CalculateSum
  (bind _values (Utilities|Map|Values (Variables|Default|GetLootTable)))
  (for _array_element _values
    (LocalVariables|SetRunningTotal (+ (LocalVariables|GetRunningTotal) _array_element)))
  (return (LocalVariables|GetRunningTotal)))

(fn ChooseLoot
  (LocalVariables|SetRandomValue (Math|Random|RandomFloatinRange 0.0 (Variables|Default|GetValueSum)))
  (bind _keys (Utilities|Map|Keys (Variables|Default|GetLootTable)))
  (for _array_element _keys
    (if (<= (LocalVariables|GetRandomValue) (.Value (Utilities|Map|Find (Variables|Default|GetLootTable) _array_element)))
      (return _array_element)
      (else
        (LocalVariables|SetRandomValue (- (LocalVariables|GetRandomValue) (.Value (Utilities|Map|Find (Variables|Default|GetLootTable) _array_element))))))))