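; BP_ReputationComponent stores per-faction reputation in a Reputations array of name and amount entries.
; Reputation_GetAmount searches the array linearly by faction name and returns the matching amount, name and index.
; Reputation_Add uses that result to write the increased amount back at the same index, with no check that the faction was found and no path for adding new factions.
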(fn ReputationAdd
  (params (Faction :type EReputation_Factions%20Enum :default "NewEnumerator0") (Amount :type Float%20%28double-precision%29))
  (bind (_currentamountofreputation _faction_name _index) (CallFunction|ReputationGetAmount Faction))
  (Utilities|Array|SetArrayElem (Variables|Default|GetReputations) _index (Utilities|Struct|MakeFReputations _faction_name (+ _currentamountofreputation Amount))))

(fn ReputationGetAmount
  (params (Name :type EReputation_Factions%20Enum :default "NewEnumerator0"))
  (bind (_array_element _array_index) (Utilities|Array|ForEachLoopwithBreak (Variables|Default|GetReputations) :!label _label)
    (:LoopBody
      (if (Utilities|Enum|Equal(Enum) (.FactionName (Utilities|Struct|BreakFReputations _array_element)) Name)
        (LocalVariables|SetbFound true)
        (goto _label Break)))
    (:Completed
      (if (LocalVariables|GetbFound)
        (return (.Amount (Utilities|Struct|BreakFReputations _array_element)) (.FactionName (Utilities|Struct|BreakFReputations _array_element)) _array_index)))))